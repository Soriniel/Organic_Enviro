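; Weather system that runs recurring rain showers with randomized start delay and duration.
; A Niagara rain effect follows the player pawn while a reversible timeline blends storm clouds, height fog and rain amount, with threshold-triggered sound fades gated by resettable DoOnce nodes.
; A second timeline drives Wetness in MPC_Weather, times the rain hold, reverses after a delay when rain ends, then schedules the next shower.
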(event Custom|Init%20Rain
  (Variables|Default|SetRainStartDelay (Math|Random|RandomFloatinRange (Variables|Default|GetRainStartDelayMin) (Variables|Default|GetRainStartDelayMax)))
  (Variables|Default|SetRainDUration (Math|Random|RandomFloatinRange (Variables|Default|GetRainDUrationMin) (Variables|Default|GetRainDUrationMax)))
  (Utilities|Time|SetTimerbyFunctionName 0 "Begin Rain" (Variables|Default|GetRainStartDelay))
  (Development|PrintString "INIT Rain"))

(event Custom|Begin%20Rain
  (Development|PrintString "Begin Rain")
  (Utilities|FlowControl|Sequence
    (:then_0
      (Components|Timeline|SetPlayRate (Variables|Default|GetRain%20Timeline) (Variables|Default|GetTransition%20Speed)))
    (:then_1
      (bind (_direction _raineffect) (Timeline|Rain%20Timeline Play)
        (:Update
          (Rendering|Material|SetScalarParameterValue (Variables|Default|GetCloudMat) "StormClouds" (Math|Float|Lerp 0.0 0.97 _raineffect) :!class /Script/Engine.MaterialInstanceDynamic)
          (Class|ExponentialHeightFogComponent|SetFogDensity (Variables|Default|GetExponentialHeightFog) (Math|Float|Lerp 0.02 1.0 _raineffect))
          (Class|ExponentialHeightFogComponent|SetFogHeightFalloff (Variables|Default|GetExponentialHeightFog) (Math|Float|Lerp 0.2 1.5 _raineffect))
          (Niagara|SetNiagaraVariable(Float) (Variables|Default|GetRainParticles) "Rain Amount" (Math|Float|MapRangeClamped _raineffect (Variables|Default|GetRain%20Min%20Alpha) (Variables|Default|GetRain%20Max%20Alpha) 0.0 1.0))
          (switch Utilities|FlowControl|Switch|SwitchonETimelineDirection _direction
            (:Forward
              (if (>= _raineffect (Variables|Default|GetRain%20Min%20Alpha))
                (Utilities|FlowControl|DoOnce false
                  (:Completed
                    (Variables|Default|GetRain%20Sound
                      (:then
                        _)
                      (:else
                        (bind _returnvalue (Audio|SpawnSound2D "/Game/SFX_Essentials_FREE_SAMPLE/SFX_Essentials_06_RAIN/Cues/RAINConc_InsJ_Ambience_Rain_Light_01_LOOP_Cue.RAINConc_InsJ_Ambience_Rain_Light_01_LOOP_Cue" 1.0 1.0 0.0 0))
                        (Variables|Default|SetRain%20Sound _returnvalue)))
                    (Audio|Components|Audio|FadeIn (Variables|Default|GetRain%20Sound) (/ 2.5 (Variables|Default|GetTransition%20Speed)) 1.0 0.0 "Linear" :!class /Script/Engine.AudioComponent)))))
            (:Backward
              (if (<= _raineffect (Variables|Default|GetRain%20Max%20Alpha))
                (Utilities|FlowControl|DoOnce false
                  (:Completed
                    (Audio|Components|Audio|FadeOut (Variables|Default|GetRain%20Sound) (/ 2.5 (Variables|Default|GetTransition%20Speed)) 0.0 "Linear" :!class /Script/Engine.AudioComponent)))))))))
    (:then_2
      (bind (_direction_2 _material_alpha) (Timeline|Material%20Time Play)
        (:Update
          (Rendering|Material|SetScalarParameterValue "/Game/Weather/MPC_Weather.MPC_Weather" "Wetness" _material_alpha :!class /Script/Engine.KismetMaterialLibrary))
        (:Finished
          (switch Utilities|FlowControl|Switch|SwitchonETimelineDirection _direction_2
            (:Forward
              (Development|PrintString "Rain Full")
              (Utilities|FlowControl|Delay (Variables|Default|GetRainDUration))
              (CallFunction|EndRain)
              (Development|PrintString "Rain End"))
            (:Backward
              (CallFunction|InitRain)
              (Development|PrintString "Rain Finished"))))))
    (:then_3
      (CallFunction|ResetDoOnceFadeOut))))

(event Custom|Reset%20Do%20Once%20Fade%20Out
  (Utilities|FlowControl|DoOnce false) ; enters at Reset
)

(event Custom|Reset%20Do%20Once%20Fade%20In
  (Utilities|FlowControl|DoOnce false) ; enters at Reset
)

(event Custom|EndRain
  (Utilities|FlowControl|Sequence
    (:then_0
      (bind (_direction _raineffect) (Timeline|Rain%20Timeline Reverse)
        (:Update
          (Rendering|Material|SetScalarParameterValue (Variables|Default|GetCloudMat) "StormClouds" (Math|Float|Lerp 0.0 0.97 _raineffect) :!class /Script/Engine.MaterialInstanceDynamic)
          (Class|ExponentialHeightFogComponent|SetFogDensity (Variables|Default|GetExponentialHeightFog) (Math|Float|Lerp 0.02 1.0 _raineffect))
          (Class|ExponentialHeightFogComponent|SetFogHeightFalloff (Variables|Default|GetExponentialHeightFog) (Math|Float|Lerp 0.2 1.5 _raineffect))
          (Niagara|SetNiagaraVariable(Float) (Variables|Default|GetRainParticles) "Rain Amount" (Math|Float|MapRangeClamped _raineffect (Variables|Default|GetRain%20Min%20Alpha) (Variables|Default|GetRain%20Max%20Alpha) 0.0 1.0))
          (switch Utilities|FlowControl|Switch|SwitchonETimelineDirection _direction
            (:Forward
              (if (>= _raineffect (Variables|Default|GetRain%20Min%20Alpha))
                (Utilities|FlowControl|DoOnce false
                  (:Completed
                    (Variables|Default|GetRain%20Sound
                      (:then
                        _)
                      (:else
                        (bind _returnvalue (Audio|SpawnSound2D "/Game/SFX_Essentials_FREE_SAMPLE/SFX_Essentials_06_RAIN/Cues/RAINConc_InsJ_Ambience_Rain_Light_01_LOOP_Cue.RAINConc_InsJ_Ambience_Rain_Light_01_LOOP_Cue" 1.0 1.0 0.0 0))
                        (Variables|Default|SetRain%20Sound _returnvalue)))
                    (Audio|Components|Audio|FadeIn (Variables|Default|GetRain%20Sound) (/ 2.5 (Variables|Default|GetTransition%20Speed)) 1.0 0.0 "Linear" :!class /Script/Engine.AudioComponent)))))
            (:Backward
              (if (<= _raineffect (Variables|Default|GetRain%20Max%20Alpha))
                (Utilities|FlowControl|DoOnce false
                  (:Completed
                    (Audio|Components|Audio|FadeOut (Variables|Default|GetRain%20Sound) (/ 2.5 (Variables|Default|GetTransition%20Speed)) 0.0 "Linear" :!class /Script/Engine.AudioComponent)))))))))
    (:then_1
      (Utilities|FlowControl|Delay (Variables|Default|GetMat%20Wetness%20DUration))
      (bind (_direction_2 _material_alpha) (Timeline|Material%20Time Reverse)
        (:Update
          (Rendering|Material|SetScalarParameterValue "/Game/Weather/MPC_Weather.MPC_Weather" "Wetness" _material_alpha :!class /Script/Engine.KismetMaterialLibrary))
        (:Finished
          (switch Utilities|FlowControl|Switch|SwitchonETimelineDirection _direction_2
            (:Forward
              (Development|PrintString "Rain Full")
              (Utilities|FlowControl|Delay (Variables|Default|GetRainDUration))
              (CallFunction|EndRain)
              (Development|PrintString "Rain End"))
            (:Backward
              (CallFunction|InitRain)
              (Development|PrintString "Rain Finished"))))))
    (:then_2
      (CallFunction|ResetDoOnceFadein))))

(event EventBeginPlay
  (Utilities|FlowControl|Sequence
    (:then_0
      (bind _returnvalue (Niagara|SpawnSystemAttached "/Game/Weather/NS_Rain.NS_Rain" (Variables|/Script/Engine.Actor|GetRootComponent (Pawn|GetControlledPawn (Game|GetPlayerController 0))) "None" "0.000000,0.000000,400.000000" "0, 0, 0" "KeepRelativeOffset" false))
      (Variables|Default|SetRainParticles _returnvalue)
      (bind _returnvalue_2 (Rendering|Material|CreateDynamicMaterialInstance (Utilities|ResolveSoftReference (Variables|/Script/Engine.VolumetricCloudComponent|GetMaterial (Variables|Default|GetVolumetricCloud))) "None" "None" :!class /Script/Engine.KismetMaterialLibrary))
      (bind _output_get (Variables|Default|SetCloudMat _returnvalue_2))
      (Rendering|Material|SetMaterial (Variables|Default|GetVolumetricCloud) _output_get))
    (:then_1
      (CallFunction|InitRain))))

(fn ConstructionScript)